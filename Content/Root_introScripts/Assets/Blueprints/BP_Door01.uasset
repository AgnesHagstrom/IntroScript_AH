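; BP_Door01 is a door that rises while something overlaps its Trigger component.
; Begin and end overlap open and close a Gate that passes Tick through to the movement.
; Each passed tick nudges Door up one unit and prints the Mover counter, which caps total travel, so speed depends on frame rate.
; Leaving the trigger pauses the door in place, and nothing lowers it again.
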(event OnComponentBeginOverlap(Trigger)
  (params (OverlappedComponent :type Primitive%20Component%20Object%20Reference) (OtherActor :type Actor%20Object%20Reference) (OtherComp :type Primitive%20Component%20Object%20Reference) (OtherBodyIndex :type Integer) (bFromSweep :type Boolean) (SweepResult :type Hit%20Result%20Structure%20%28by%20ref%29))
  (Utilities|FlowControl|Gate true) ; enters at Open
)

(event OnComponentEndOverlap(Trigger)
  (params (OverlappedComponent :type Primitive%20Component%20Object%20Reference) (OtherActor :type Actor%20Object%20Reference) (OtherComp :type Primitive%20Component%20Object%20Reference) (OtherBodyIndex :type Integer))
  (Utilities|FlowControl|Gate true) ; enters at Close
)

(event EventTick
  (params (DeltaSeconds :type Float%20%28single-precision%29))
  (Utilities|FlowControl|Gate true
    (:Exit
      (if (not (>= (Variables|Default|GetMover) 3e+02))
        (bind _result (Math|Float|IncrementFloat (Variables|Default|GetMover))
          (:%20%20
            (Variables|Default|SetMover _result)
            (Transformation|AddLocalOffset (Variables|Default|Getdoor) (Math|Vector|MakeVector 0.0 0.0 1.0) false false)
            (Development|PrintString (Utilities|String|ToString(Float) (Variables|Default|GetMover)))))))))

(fn ConstructionScript)